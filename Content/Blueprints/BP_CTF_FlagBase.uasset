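; Capture-the-flag base actor that spawns and respawns the flag for its assigned team.
; On BeginPlay it spawns a flag at its Billboard transform, passing itself as the base reference, plus a capture point owned by the opposing team.
; Reset_The_Flag returns the flag home by destroying the stored instance and spawning a fresh one rather than moving it.
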(event `self.ReceiveBeginPlay`
  (bind _team (`self.Team`))
  (bind _returnvalue (`SceneComponent.K2_GetComponentToWorld` (`self.Billboard`)))
  ;[1 1 1] On start get our team and set colors
  (bind _returnvalue_2 (`|SpawnActorFromClass` "/CTF_GameMode/Blueprints/BP_CTF_Flag.BP_CTF_Flag_C" _returnvalue "Undefined" "OverrideRootScale" null _team self))
  (set `self.Flag_Reference` _returnvalue_2)
  (if (`|EnumEquality` _team "Team_One")
    (`|SpawnActorFromClass` "/CTF_GameMode/Blueprints/BP_CTF_FlagCapturePoint.BP_CTF_FlagCapturePoint_C" _returnvalue "Undefined" "OverrideRootScale" null 0 "Team_Two")
    (else
      (`|SpawnActorFromClass` "/CTF_GameMode/Blueprints/BP_CTF_FlagCapturePoint.BP_CTF_FlagCapturePoint_C" _returnvalue "Undefined" "OverrideRootScale" null 0 "Team_One"))))

(event `Reset_The_Flag`
  ;[1 1 1] Reset the Flag to Home
  (`self.K2_DestroyActor` (`self.Flag_Reference`))
  (bind _returnvalue (`|SpawnActorFromClass` "/CTF_GameMode/Blueprints/BP_CTF_Flag.BP_CTF_Flag_C" (`SceneComponent.K2_GetComponentToWorld` (`self.Billboard`)) "Undefined" "OverrideRootScale" null (`self.Team`) self))
  (set `self.Flag_Reference` _returnvalue))

(fn `UserConstructionScript`)