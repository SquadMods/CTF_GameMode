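; BP_CTF_FlagCapturePoint is the team-owned point where flags are captured in Capture the Flag.
; On BeginPlay it sets the Cylinder's material according to its owning team.
; When an overlapping BP_CTF_Flag has the same OwningTeam as the point, it reports the capture for that team to BP_GameMode_CTF.
; It then calls FlagCaptured on the flag to send it home.
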(event `self.ReceiveBeginPlay`
  (bind _cylinder (`self.Cylinder`))
  ;[1 1 1] Set color based on team at start
  (switch `ESQTeam` (`self.Owning_Team`)
    (:`Team_One`
      (`PrimitiveComponent.SetMaterial` _cylinder 0 null))
    (:`Team_Two`
      (`PrimitiveComponent.SetMaterial` _cylinder 0 null))))

(event `self.ReceiveActorBeginOverlap`
  (params (OtherActor :type "Actor Object Reference"))
  ;[1 1 1] If a friendly flag touches us, then let the gamemode know that we capped and reset the flag to it's home.
  (bind _asbp_ctf_flag (cast `/CTF_GameMode/Blueprints/BP_CTF_Flag` OtherActor))
  (if (`|EnumEquality` (`/CTF_GameMode/Blueprints/BP_CTF_Flag.Owning_Team` _asbp_ctf_flag) (`self.Owning_Team`))
    (bind _asbp_game_mode_ctf (cast `/CTF_GameMode/Gameplay/GameModes/BP_GameMode_CTF` (`GameplayStatics.GetGameMode`)))
    (`/CTF_GameMode/Gameplay/GameModes/BP_GameMode_CTF.FlagCaptured` _asbp_game_mode_ctf (`self.Owning_Team`))
    (`/CTF_GameMode/Blueprints/BP_CTF_Flag.Flag_Captured` _asbp_ctf_flag)))

(fn `UserConstructionScript`)