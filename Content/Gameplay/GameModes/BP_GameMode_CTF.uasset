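; Capture the Flag game mode that tracks flag captures for two teams and ends the match when either reaches the capture limit.
; FlagCaptured increments the scoring team's counter, then CheckForMatchEnd compares both counters to MaxFlagCaptures and calls EndMatch.
; BeginPlay only calls the parent, and unconnected nodes for looping over team players and casting their HUDs never run.
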(event `self.ReceiveBeginPlay`
  (`parent.ReceiveBeginPlay`))

(event `FlagCaptured`
  (params (Team :type "ESQTeam Enum"))
  (switch `ESQTeam` Team
    (:`Team_One`
      (`/Engine/EditorBlueprintResources/StandardMacros.IncrementInt` (`self.TeamOneFlagCaptures`)
        (:`  `
          _)))
    (:`Team_Two`
      (`/Engine/EditorBlueprintResources/StandardMacros.IncrementInt` (`self.TeamTwoFlagCaptures`)
        (:`  `
          _))))
  (`self.CheckForMatchEnd`))

(event `CheckForMatchEnd`
  (bind _maxflagcaptures (`self.MaxFlagCaptures`))
  (if (not (and (< (`self.TeamOneFlagCaptures`) _maxflagcaptures) (< (`self.TeamTwoFlagCaptures`) _maxflagcaptures)))
    (`self.EndMatch`)))

(fn `UserConstructionScript`
  (`parent.UserConstructionScript`))